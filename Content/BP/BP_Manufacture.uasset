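; BP_Manufacture is a crafting station actor that turns three planks into a table.
; Box overlaps add each BP_Plank to an array and increment a counter.
; When the count equals three, it destroys the stored planks and spawns a BP_Table offset along world X, without resetting array or counter.
; End overlap does nothing, as its removal logic is disconnected, so planks leaving the box stay counted.
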(event OnComponentBeginOverlap(Box)
  (params (OverlappedComponent :type Primitive%20Component%20Object%20Reference) (OtherActor :type Actor%20Object%20Reference) (OtherComp :type Primitive%20Component%20Object%20Reference) (OtherBodyIndex :type Integer) (bFromSweep :type Boolean) (SweepResult :type Hit%20Result%20Structure%20%28by%20ref%29))
  (bind _returnvalue (Transformation|GetActorTransform))
  (bind _planks (Variables|Default|GetPlanks))
  (bind _asbp_plank (Utilities|Casting|CastToBP_Plank OtherActor))
  (Utilities|Array|Add _planks _asbp_plank)
  (Variables|Default|SetCountPlank (+ (Variables|Default|GetCountPlank) 1))
  (if (== (Variables|Default|GetCountPlank) 3)
    (for _array_element _planks
      (Actor|DestroyActor _array_element))
    (Game|SpawnActorfromClass "/Game/BP/BP_Table.BP_Table_C" (Math|Transform|MakeTransform (Math|Vector|MakeVector (- (.x (.location _returnvalue)) 1e+02) (.y (.location _returnvalue)) (.z (.location _returnvalue))) (.rotation _returnvalue) (.scale _returnvalue)) "Undefined" "MultiplyWithRoot" 0 0)))

(event OnComponentEndOverlap(Box)
  (params (OverlappedComponent :type Primitive%20Component%20Object%20Reference) (OtherActor :type Actor%20Object%20Reference) (OtherComp :type Primitive%20Component%20Object%20Reference) (OtherBodyIndex :type Integer)))

(fn ConstructionScript)